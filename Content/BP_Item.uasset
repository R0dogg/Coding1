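; BP_Item is an item Blueprint with a name, an elemental type and type-based damage, reported through debug prints on BeginPlay.
; Constructor shuffles a literal four-name array but reads Name from a rebuilt copy's first element, so the shuffle has no effect.
; GetDamage doubles Damage when the victim's type index plus two, modulo five, equals the item's own.
; BeginPlay tests this against a fixed victim type, labeled air.
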(event `self.ReceiveBeginPlay`
  (`self.Constructor`)
  (`KismetSystemLibrary.PrintString` (`KismetStringLibrary.Concat_StrStr` "Hello! My name is " (`self.Name`)) true true (struct :`G` 0.66 :`B` 1.0 :`A` 1.0) 30.0)
  (bind _damage (`self.Get Damage` "NewEnumerator3"))
  (`KismetSystemLibrary.PrintString` (`KismetStringLibrary.Concat_StrStr` "Our elemental type is  " (`|GetEnumeratorNameAsString` (`self.ElementalType`)) ",  victim is air, damage = " (`KismetStringLibrary.Conv_IntToString` _damage)) true true (struct :`G` 0.66 :`B` 1.0 :`A` 1.0) 30.0))

(fn `Constructor`
  (bind _array (`|MakeArray` "Roman" "Julie" "Tom" "Jillian"))
  (`KismetArrayLibrary.Array_Shuffle` _array)
  (set `self.Name` (`|GetArrayItem` _array)))

(fn `Get Damage`
  (params (`Victim Elem Type` :type "/Game/ElementalType Enum" :default "NewEnumerator0"))
  (returns (Damage :type Integer))
  (locals (`Returned Damage` :type Integer))
  (set `local.Returned Damage` (`self.Damage`))
  (if (== (mod (+ `Victim Elem Type` 2) 5) (`KismetMathLibrary.Conv_ByteToInt` (`self.ElementalType`)))
    (set `local.Returned Damage` (* (`self.Damage`) 2)))
  (return (`local.Returned Damage`)))

(fn `UserConstructionScript`)