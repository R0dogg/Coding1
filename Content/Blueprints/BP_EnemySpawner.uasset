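; BP_EnemySpawner spawns BP_Enemy actors at the level's BP_EnemySpawnLocation actors.
; On BeginPlay it gathers and prints the location count, then spawns a wave, with a random roll letting most locations produce an enemy.
; A self-calling check repeats on a delay and spawns another wave when its actor query returns empty, though that query has no class set.
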(event `self.ReceiveBeginPlay`
  (bind _outactors (`GameplayStatics.GetAllActorsOfClass` "/Game/Blueprints/BP_EnemySpawnLocation.BP_EnemySpawnLocation_C"))
  (`KismetSystemLibrary.PrintString` (`KismetStringLibrary.Concat_StrStr` "There are " (`KismetStringLibrary.Conv_IntToString` (`KismetArrayLibrary.Array_Length` _outactors)) " spawners in the level"))
  (`self.Spawn Enemies`)
  (`self.Enemy Count Check`))

(event `Spawn Enemies`
  (for _array_element (stale `self.ReceiveBeginPlay` _outactors)
    (if (> (`KismetMathLibrary.RandomFloat`) 0.2)
      (`|SpawnActorFromClass` "/Game/Blueprints/BP_Enemy.BP_Enemy_C" (`self.GetTransform` _array_element) "Undefined" "MultiplyWithRoot" null null))))

(event `Enemy Count Check`
  (bind _outactors (`GameplayStatics.GetAllActorsOfClass` null))
  (if (not (> (`KismetArrayLibrary.Array_Length` _outactors) 0))
    (`self.Spawn Enemies`))
  (`KismetSystemLibrary.Delay` 2.0)
  (`self.Enemy Count Check`))

(fn `UserConstructionScript`)