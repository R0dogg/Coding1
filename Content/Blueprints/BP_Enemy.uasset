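; BP_Enemy is an enemy actor that takes on a name and team material and is destroyed when the third-person character touches it.
; On BeginPlay it fills an unset name from a shuffled list, picks a random material if none is assigned, and applies it to the Body.
; Capsule overlap with the player sets Health negative, and a looping Delay polls Health to destroy the actor, avoiding Tick.
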(event `self.ReceiveBeginPlay`
  (bind _names (`self.Names`))
  (bind _newvar (`self.NewVar`))
  (`|ExecutionSequence`
    (:`then_0`
      (`KismetSystemLibrary.Delay` 0.2 :!label _label)
      (if (<= (`self.Health`) 0.0)
        (`self.K2_DestroyActor`)
        (else
          (goto _label))))
    (:`then_1`
      (if (== (`self.Enemy Name`) "None")
        (`KismetArrayLibrary.Array_Shuffle` _names)
        (set `self.Enemy Name` (`|GetArrayItem` _names)))
      (`KismetSystemLibrary.PrintString` (`KismetStringLibrary.Concat_StrStr` (`KismetStringLibrary.Conv_NameToString` (`self.Enemy Name`)) " exists!")))
    (:`then_2`
      (`/Engine/EditorBlueprintResources/StandardMacros.IsValid` (`self.Enemy Team Material`)
        (:`Is Valid`
          (`KismetSystemLibrary.PrintString` "A material has been set"))
        (:`Is Not Valid`
          (`KismetSystemLibrary.PrintString` "Let's pick a random material")
          (`KismetArrayLibrary.Array_Shuffle` _newvar)
          (set `self.Enemy Team Material` (`|GetArrayItem` _newvar))))
      (`PrimitiveComponent.SetMaterial` (`self.body`) 0 (`self.Enemy Team Material`)))))

(event `self.Capsule.OnComponentBeginOverlap`
  (params (OverlappedComponent :type "PrimitiveComponent Object Reference") (OtherActor :type "Actor Object Reference") (OtherComp :type "PrimitiveComponent Object Reference") (OtherBodyIndex :type Integer) (bFromSweep :type Boolean) (SweepResult :type "HitResult Structure (by ref)"))
  (cast `/Game/ThirdPerson/Blueprints/BP_ThirdPersonCharacter` OtherActor)
  (set `self.Health` -1.0))

(fn `UserConstructionScript`)