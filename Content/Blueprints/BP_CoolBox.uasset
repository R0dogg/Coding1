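; BP_CoolBox is an actor that endlessly spawns BP_Key actors above its Cube component.
; On BeginPlay it stores a spawn point at a fixed height over the cube and prints debug messages with its name and that location.
; It then spawns a randomly scaled key, waits SpawnDelay and loops back through the Delay node to repeat without a timer or Tick.
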(event `self.ReceiveBeginPlay`
  (set `self.KeySpawnLocation` (+ (`SceneComponent.K2_GetComponentLocation` (`self.Cube`)) (0.0 0.0 800.0)))
  (`KismetSystemLibrary.PrintString` (`KismetStringLibrary.Concat_StrStr` (`KismetSystemLibrary.GetDisplayName` self) " is the best!") true true (struct :`G` 0.04179 :`B` 0.097222 :`A` 1.0) 10.0)
  (`KismetSystemLibrary.PrintString` (`KismetStringLibrary.Conv_VectorToString` (`self.KeySpawnLocation`)))
  (`KismetSystemLibrary.PrintString` (`KismetStringLibrary.Conv_VectorToString` (`self.KeySpawnLocation`)))
  (`|SpawnActorFromClass` "/Game/Blueprints/BP_Key.BP_Key_C" (`KismetMathLibrary.MakeTransform` (`self.KeySpawnLocation`) (struct) (* 1.0 (`KismetMathLibrary.RandomFloatInRange` 0.1 2.0))) "Undefined" "MultiplyWithRoot" null null :!label _label)
  (`KismetSystemLibrary.Delay` (`self.SpawnDelay`))
  (goto _label))

(fn `UserConstructionScript`)